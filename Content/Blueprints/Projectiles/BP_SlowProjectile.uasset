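; BP_SlowProjectile is a projectile that holds off homing for a delay, then launches at its homing target.
; DelayAttack disables homing, waits, then, if the target component is valid, re-enables weak homing and sets a five-second lifespan.
; The launch velocity is an intercept vector toward the target's owner, with speed set to distance divided by the requested homing time.
; The velocity calculation also draws a debug arrow along that vector.
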(event Custom|Delay%20Attack
  (params (Delay :type Float%20%28double-precision%29) (Homing%20Time :type Float%20%28double-precision%29))
  (Variables|/Script/Engine.ProjectileMovementComponent|SetbIsHomingProjectile (Variables|Default|GetProjectileComponent) false)
  (Utilities|FlowControl|Delay Delay)
  (Utilities|IsValid (Variables|/Script/Engine.ProjectileMovementComponent|GetHomingTargetComponent (Variables|Default|GetProjectileComponent))
    (:Is%20Valid
      (Variables|/Script/Engine.ProjectileMovementComponent|SetbIsHomingProjectile (Variables|Default|GetProjectileComponent) true)
      (Variables|/Script/Engine.MovementComponent|SetVelocity (Variables|Default|GetProjectileComponent) (CallFunction|CalculateHomingFireVelocity Homing%20Time))
      (Variables|/Script/Engine.ProjectileMovementComponent|SetHomingAccelerationMagnitude (Variables|Default|GetProjectileComponent) 1e+01)
      (Actor|SetLifeSpan 5.0))))

(event EventBeginPlay)

(fn ConstructionScript)

(fn CalculateHomingFireVelocity
  (params (Homing%20Time :type Float%20%28double-precision%29))
  (bind _returnvalue (Transformation|GetActorLocation))
  (bind _returnvalue_2 (Transformation|GetActorLocation))
  (bind _projectilecomponent (Variables|Default|GetProjectileComponent))
  (bind _homingtargetcomponent (Variables|/Script/Engine.ProjectileMovementComponent|GetHomingTargetComponent _projectilecomponent))
  (bind _returnvalue_3 (Components|GetOwner _homingtargetcomponent))
  (bind _returnvalue_4 (Transformation|GetActorLocation _returnvalue_3))
  (bind _returnvalue_5 (Math|Vector|Distance(Vector) _returnvalue_2 _returnvalue_4))
  (bind _returnvalue_6 (Math|Float|SafeDivide _returnvalue_5 Homing%20Time))
  (bind _returnvalue_7 (Class|TargetingUtils|CalculateInterceptVector 0 _returnvalue_3 _returnvalue_6))
  (Rendering|Debug|DrawDebugArrow :LineStart _returnvalue :LineEnd (+ _returnvalue _returnvalue_7) :ArrowSize 1e+01 :Duration 5.0 :Thickness 5.0)
  (return _returnvalue_7))

(fn GetInitialVelocity
  (return (Variables|/Script/Engine.MovementComponent|GetVelocity (Variables|Default|GetProjectileComponent))))