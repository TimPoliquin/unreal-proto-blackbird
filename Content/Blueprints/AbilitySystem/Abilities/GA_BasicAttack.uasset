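; GA_BasicAttack is a gameplay ability for a basic ranged attack from the primary left weapon socket.
; On activation it commits, cancelling if that fails, then waits for target data under the mouse.
; When a mouse target arrives, it spawns a projectile toward the hit point and actor, then ends.
; It also reports a fixed heat cost that ignores level.
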(event Ability|EventActivateAbility
  (bind _returnvalue (Ability|CommitAbility))
  (if _returnvalue
    (bind _datahandle (|TargetDataUnderMouse)
      (:HasMouseTarget
        (Class|BlackbirdProjectileAbility|SpawnProjectile (GameplayTags|MakeLiteralGameplayTag "(TagName=\"Actor.Socket.Weapon.Primary.Left\")") (.ImpactPoint (Collision|BreakHitResult (Ability|TargetData|GetHitResultfromTargetData _datahandle))) (.HitActor (Collision|BreakHitResult (Ability|TargetData|GetHitResultfromTargetData _datahandle))))
        (Ability|EndAbility)))
    (else
      (Ability|CancelAbility))))

(fn GetHeatCost
  (params (InLevel :type Float%20%28single-precision%29))
  (return 1.0))