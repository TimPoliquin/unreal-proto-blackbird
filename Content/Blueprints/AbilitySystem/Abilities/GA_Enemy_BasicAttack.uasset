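; Gameplay ability for a basic enemy attack that fires a projectile at the player's ship.
; On a successful commit, it spawns the projectile from the left primary weapon socket, targeting the first BlackbirdPlayerShip found in the world without a validity check.
; A BP_SlowProjectile gets a delayed attack with a homing time, and the ability ends immediately.
; A failed commit cancels it; heat cost is flat across levels.
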(event Ability|EventActivateAbility
  (bind _returnvalue (Ability|CommitAbility))
  (if _returnvalue
    (bind _outactors (Actor|GetAllActorsOfClass "/Script/Blackbird.BlackbirdPlayerShip"))
    (bind _returnvalue_2 (Class|BlackbirdProjectileAbility|SpawnProjectile (GameplayTags|MakeLiteralGameplayTag "(TagName=\"Actor.Socket.Weapon.Primary.Left\")") (Transformation|GetActorLocation (Utilities|Array|Get(acopy) _outactors)) (Utilities|Array|Get(acopy) _outactors) true))
    (bind _asbp_slow_projectile (Utilities|Casting|CastToBP_SlowProjectile _returnvalue_2)
      (:then
        (Default|DelayAttack _asbp_slow_projectile 4.0 2.0)
        (Ability|EndAbility))
      (:CastFailed
        (Ability|EndAbility)))
    (else
      (Ability|CancelAbility)
      (Development|PrintString "Cancelled"))))

(fn GetHeatCost
  (params (InLevel :type Float%20%28single-precision%29))
  (return 1.0))