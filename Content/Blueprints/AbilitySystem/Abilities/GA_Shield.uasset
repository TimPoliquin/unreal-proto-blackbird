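; GA_Shield is a hold-to-use gameplay ability that shields its owner while the input is held, at a recurring heat cost.
; On activation it draws a debug sphere, applies GE_Shielded and starts a looping timer that commits the ability cost each second.
; Releasing input ends the ability, which removes the effect, commits the cooldown and clears the timer.
; GetHeatCost returns a fixed cost regardless of level.
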(event Custom|Event%20Commit%20Cost
  (Ability|CommitAbilityCost false))

(event Ability|EventActivateAbility
  (Rendering|Debug|DrawDebugSphere (Transformation|GetActorLocation (Ability|GetAvatarActorfromActorInfo)) 1e+02 12 "(R=0.062289,G=1.000000,B=0.000000,A=1.000000)" 0.0 2.0)
  (bind _returnvalue (Ability|ApplyGameplayEffectToOwner "/Game/Blueprints/AbilitySystem/Effects/StatusEffect/GE_Shielded.GE_Shielded_C"))
  (Variables|Default|SetShield%20Effect _returnvalue)
  (Ability|Tasks|WaitInputRelease false
    (:then
      (bind _returnvalue_2 (Utilities|Time|SetTimerbyEvent (delegate Custom|Event%20Commit%20Cost) 1.0 true))
      (Variables|Default|SetCommit%20Timer _returnvalue_2))
    (:OnRelease
      (Ability|EndAbility))))

(event Ability|EventOnEndAbility
  (params (bWasCancelled :type Boolean))
  (Ability|RemoveGameplayEffectFromOwnerWithHandle (Variables|Default|GetShield%20Effect))
  (Ability|CommitAbilityCooldown true)
  (Utilities|Time|ClearandInvalidateTimerbyHandle (Variables|Default|GetCommit%20Timer)))

(fn GetHeatCost
  (params (InLevel :type Float%20%28single-precision%29))
  (return 2.0))