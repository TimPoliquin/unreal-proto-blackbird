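; GA_Repel is a gameplay ability that deflects nearby projectiles, making the avatar their new owner.
; On activation it sphere-overlaps around the avatar for projectiles within Radius, drawing a debug sphere.
; If any are found, it runs one long-range target trace and sends each projectile a RepelMessage with that target, the repel angle and doubled base damage.
; The ability ends immediately either way.
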(event Ability|EventActivateAbility
  (bind (_targets _has_targets) (CallFunction|FindProjectilesinRange))
  (if _has_targets
    (bind _outhitresult (CallFunction|FindRepelDirection))
    (for _array_element _targets
      (CallFunction|RepelProjectile _array_element _outhitresult))
    (Ability|EndAbility)
    (else
      (Ability|EndAbility))))

(event Ability|EventOnEndAbility
  (params (bWasCancelled :type Boolean)))

(fn FindProjectilesinRange
  (bind _returnvalue (Ability|GetAvatarActorfromActorInfo))
  (bind _returnvalue_2 (Transformation|GetActorLocation _returnvalue))
  (bind (_outactors _returnvalue_3) (Collision|SphereOverlapActors _returnvalue_2 (Variables|Default|GetRadius) (Utilities|Array|MakeArray "ObjectTypeQuery7") 0 (Utilities|Array|MakeArray _returnvalue)))
  (Rendering|Debug|DrawDebugSphere _returnvalue_2 (Variables|Default|GetRadius) 12 "(R=1.000000,G=1.000000,B=1.000000,A=1.000000)" 1.0 1.0)
  (return _outactors _returnvalue_3))

(fn FindRepelDirection
  (return (Class|TargetingUtils|FindActorTarget (Ability|GetAvatarActorfromActorInfo) 1e+04 false)))

(fn RepelProjectile
  (params (Projectile :type Actor%20Object%20Reference) (Hit%20Result :type Hit%20Result%20Structure))
  (Actor|SetOwner Projectile (Ability|GetAvatarActorfromActorInfo))
  (Class|ProjectileInterface|Repel(Message) Projectile (Ability|GetAvatarActorfromActorInfo) Hit%20Result (Variables|Default|GetRepel%20Angle) 2.0))