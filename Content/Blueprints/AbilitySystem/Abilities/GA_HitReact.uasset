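; GA_HitReact is a gameplay ability that plays a directional hit reaction on the Blackbird player.
; On activation it applies the GE_HitReact effect to the avatar and plays AM_HitReact, choosing the left or right section from the Y sign of the player's ReactionDirection.
; The ability ends when the montage completes, blends out or is cut short, removing the effect by its stored handle.
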(event Ability|EventActivateAbility
  (bind _returnvalue (Class|BlackbirdAbilitySystemLibrary|ApplyEffecttoSelf (Ability|GetAvatarActorfromActorInfo) "/Game/Blueprints/AbilitySystem/Effects/Block/GE_HitReact.GE_HitReact_C" 1 0.0))
  (Variables|Default|SetHit%20React%20Effect _returnvalue)
  (|PlayMontageandWaitProxy "HitReact" "/Game/Blueprints/Player/Animation/AM_HitReact.AM_HitReact" 1.0 (CallFunction|DetermineHitReactMontage) true 1.0 0.0 false
    (:OnCompleted
      (Ability|EndAbility))
    (:OnBlendOut
      (Ability|EndAbility))
    (:OnInterrupted
      (Ability|EndAbility))
    (:OnCancelled
      (Ability|EndAbility))))

(event Ability|EventOnEndAbility
  (params (bWasCancelled :type Boolean))
  (Ability|RemoveGameplayEffectFromOwnerWithHandle (Variables|Default|GetHit%20React%20Effect)))

(fn DetermineHitReactMontage
  (bind _asbp_blackbird_player (Utilities|Casting|CastToBP_BlackbirdPlayer (Ability|GetAvatarActorfromActorInfo)))
  (if (> (.y (Variables|/Game/Blueprints/Player/BP_BlackbirdPlayer.BP_BlackbirdPlayer_C|GetReaction%20Direction _asbp_blackbird_player)) 0.0)
    (LocalVariables|SetHit%20React%20Section "HitReact_Right")
    (else
      (LocalVariables|SetHit%20React%20Section "HitReact_Left")))
  (return (LocalVariables|GetHit%20React%20Section)))