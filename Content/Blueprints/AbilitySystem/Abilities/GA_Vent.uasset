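; GA_Vent is a hold-to-vent Gameplay Ability that spends heat and triggers the Repel ability on activation.
; If usable heat (max minus available) covers the initial cost, it applies cost, vent and passive-regen-block effects.
; It ends on input release or when an Available Heat change leaves the value at or below the tick cost.
; Ending removes the vent and block effects by stored handle.
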(event Custom|Event%20OnAvatarActorAttributeChanged
  (params (Attribute :type Gameplay%20Attribute%20Structure%20%28by%20ref%29) (AttributeTag :type Gameplay%20Tag%20Structure%20%28by%20ref%29) (NewValue :type Float%20%28single-precision%29))
  (|SwitchGameplayTag AttributeTag
    (:Attributes.Vital.AvailableHeat
      (if (not (> NewValue (Variables|Default|GetHeat%20Tick%20Cost)))
        (Ability|EndAbility)))))

(event Ability|EventActivateAbility
  (if (>= (CallFunction|GetUsableHeat) (Variables|Default|GetHeat%20Initial%20Cost))
    (CallFunction|ApplyCost)
    (CallFunction|ApplyBlockPassiveHeatRegen)
    (CallFunction|ApplyVentHeatEffect)
    (CallFunction|TriggerRepelAbility)
    (Ability|Tasks|WaitInputRelease true
      (:then
        (bind _returnvalue (GameplayAttributes|GetAttributeSet (Ability|GetAbilitySystemComponent (Ability|GetAvatarActorfromActorInfo)) "/Script/Blackbird.BlackbirdBasicAttributeSet"))
        (EventDispatchers|AssignOnAttributeChanged _returnvalue (delegate Custom|Event%20OnAvatarActorAttributeChanged)))
      (:OnRelease
        (Ability|EndAbility)))
    (else
      (Ability|EndAbility))))

(event Ability|EventOnEndAbility
  (params (bWasCancelled :type Boolean))
  (Ability|RemoveGameplayEffectFromOwnerWithHandle (Variables|Default|GetVent%20Heat%20Effect))
  (Ability|RemoveGameplayEffectFromOwnerWithHandle (Variables|Default|GetBlock%20Heat%20Regen%20Effect))
  (Ability|RemoveGameplayEffectFromOwnerWithHandle))

(fn GetUsableHeat
  (bind _returnvalue (GameplayAttributes|GetAttributeSet (Ability|GetAbilitySystemComponent (Ability|GetAvatarActorfromActorInfo)) "/Script/Blackbird.BlackbirdAttributeSet"))
  (return (- (.CurrentValue (Utilities|Struct|BreakGameplayAttributeData (Variables|/Script/Blackbird.BlackbirdAttributeSet|GetMaxHeat _returnvalue))) (.CurrentValue (Utilities|Struct|BreakGameplayAttributeData (Variables|/Script/Blackbird.BlackbirdAttributeSet|GetAvailableHeat _returnvalue))))))

(fn ApplyBlockPassiveHeatRegen
  (bind _returnvalue (Class|BlackbirdAbilitySystemLibrary|ApplyEffecttoSelf (Ability|GetAvatarActorfromActorInfo) "/Game/Blueprints/AbilitySystem/Effects/Block/GE_Block_Passive_HeatCooldown.GE_Block_Passive_HeatCooldown_C" 1 0.0))
  (Variables|Default|SetBlock%20Heat%20Regen%20Effect _returnvalue))

(fn ApplyVentHeatEffect
  (bind _returnvalue (Class|BlackbirdAbilitySystemLibrary|ApplyEffecttoSelf (Ability|GetAvatarActorfromActorInfo) "/Game/Blueprints/AbilitySystem/Effects/StatusEffect/GE_VentHeat.GE_VentHeat_C" 1 0.0))
  (Variables|Default|SetVent%20Heat%20Effect _returnvalue))

(fn ApplyCost
  (Class|BlackbirdAbilitySystemLibrary|ApplyEffecttoSelf (Ability|GetAvatarActorfromActorInfo) "/Game/Blueprints/AbilitySystem/Effects/Cost/GE_VentHeat_Cost.GE_VentHeat_Cost_C" 1 0.0))

(fn TriggerRepelAbility
  (Abilities|TryActivateAbilitiesbyTag (Ability|GetAbilitySystemComponent (Ability|GetAvatarActorfromActorInfo)) (GameplayTags|MakeGameplayTagContainerfromTag "(TagName=\"Abilities.Ability.Repel\")") true))