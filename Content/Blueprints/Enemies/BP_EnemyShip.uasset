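; Enemy ship Blueprint that shows a health widget and explodes when killed.
; Once its Blackbird ability system is ready, it sets itself as owner of the health widget and binds to the attribute set's received-damage delegate.
; A fatal hit spawns a Niagara explosion at the ship's location and destroys the actor.
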(event Custom|OnAbilitySystemReadyDelegate_Event
  (params (BlackbirdAbilitySystemComponent :type Blackbird%20Ability%20System%20Component%20Object%20Reference))
  (CallFunction|InitializeAttributesWidget)
  (EventDispatchers|AssignOnReceivedDamage (Class|BlackbirdShip|GetBlackbirdAttributeSet) (delegate Custom|OnReceivedDamage_Event)))

(event Custom|OnReceivedDamage_Event
  (params (DamageAmount :type Float%20%28single-precision%29) (bFatal :type Boolean))
  (if bFatal
    (CallFunction|Die)))

(event EventBeginPlay
  (EventDispatchers|AssignOnAbilitySystemReadyDelegate (delegate Custom|OnAbilitySystemReadyDelegate_Event)))

(event Collision|EventActorBeginOverlap
  (params (OtherActor :type Actor%20Object%20Reference)))

(event EventTick
  (params (DeltaSeconds :type Float%20%28single-precision%29)))

(fn ConstructionScript)

(fn InitializeAttributesWidget
  (bind _aswbp_enemy_health (Utilities|Casting|CastToWBP_EnemyHealth (UserInterface|GetWidget (Variables|Default|GetAttributesWidget))))
  (Default|SetOwner _aswbp_enemy_health self))

(fn Die
  (Niagara|SpawnSystematLocation "/Game/Blueprints/Projectiles/NS_Explosion.NS_Explosion" (Transformation|GetActorLocation))
  (Actor|DestroyActor))