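; Enemy track actor for the demo level that spawns and directs a squadron along a spline.
; StartTrack spawns the squadron class at the spline's first point, hands it the Track, stores it and calls Spawn.
; The Trigger02Attack track event tells a valid squadron to attack, while the Trigger01Engage event is bound but empty.
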(event OnTrackEventTriggeredDelegate(Trigger-01-Engage)
  (params (TriggeringActor :type Actor%20Object%20Reference) (Data :type Blackbird%20Track%20Event%20Triggered%20Payload%20Structure%20%28by%20ref%29)))

(event OnTrackEventTriggeredDelegate(Trigger-02-Attack)
  (params (TriggeringActor :type Actor%20Object%20Reference) (Data :type Blackbird%20Track%20Event%20Triggered%20Payload%20Structure%20%28by%20ref%29))
  (bind _squadron (Variables|Default|GetSquadron)
    (:then
      (Default|OnAttack _squadron))
    (:else)))

(event Custom|Start%20Track
  (bind _squadron (CallFunction|SpawnSquadronActor))
  (bind _output_get (Variables|Default|SetSquadron _squadron))
  (Class|BlackbirdSquadron|Spawn _output_get))

(event EventBeginPlay)

(event Collision|EventActorBeginOverlap
  (params (OtherActor :type Actor%20Object%20Reference)))

(event EventTick
  (params (DeltaSeconds :type Float%20%28single-precision%29)))

(fn ConstructionScript)

(fn SpawnSquadronActor
  (bind _returnvalue (Game|SpawnActorfromClass (Variables|Default|GetSquadron%20Class) (Spline|GetTransformatSplinePoint (Variables|Default|GetTrack) 0 "World" false) "Undefined" "MultiplyWithRoot" self 0))
  (Class|BlackbirdSquadron|SetTrack _returnvalue (Variables|Default|GetTrack))
  (return _returnvalue))