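; Track event actor that spawns an enemy or ally squadron when a track keyframe tagged Start fires and sends it away on the End tag.
; It spawns a BP_Cart at the entrance spline and attaches an actor of the configured squadron class to it.
; Track-completion callbacks move the cart from entrance to main track, and End switches it to the exit spline, where finishing destroys the cart hierarchy.
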(event Custom|On%20Spawn%20Squadron
  (bind _cart (CallFunction|SpawnSquadronCart))
  (bind _output_get (Variables|Default|SetCart _cart))
  (bind _squadron (CallFunction|SpawnSquadronActor _output_get))
  (Variables|Default|SetSquadron _squadron)
  (EventDispatchers|AssignOnTrackCompleted (Variables|/Script/Blackbird.BlackbirdCart|GetTrackComponent (Variables|Default|GetCart)) (delegate Custom|On%20Track%20Completed)))

(event Custom|On%20End%20Squadron
  (Class|BlackbirdCart|SwitchtoTrack (Variables|Default|GetCart) (Variables|Default|GetExit%20Spline))
  (Class|BlackbirdCart|ChangeSpeed (Variables|Default|GetCart) (Variables|Default|GetExit%20Speed)))

(event Custom|On%20Track%20Completed
  (params (Cart :type Actor%20Object%20Reference) (Track :type Spline%20Component%20Object%20Reference) (Overflow :type Float%20%28single-precision%29))
  (if (== Track (Variables|Default|GetEntrance%20Spline))
    (CallFunction|OnEntranceTrackCompleted)
    (elif (== Track (Variables|Default|GetExit%20Spline))
      (CallFunction|OnExitTrackCompleted))))

(event Custom|On%20Entrance%20Track%20Completed
  (Class|BlackbirdCart|SwitchtoTrack (Variables|Default|GetCart) (Class|BlackbirdTrack|GetTrack (Variables|Default|GetMain%20Track)))
  (Class|BlackbirdCart|ChangeSpeed (Variables|Default|GetCart) (Variables|Default|GetTravel%20Speed)))

(event Custom|On%20Exit%20Track%20Completed
  (Class|ActorFunctionLibrary|DestroyActorHierarchy (Variables|Default|GetCart)))

(event EventBeginPlay)

(event Collision|EventActorBeginOverlap
  (params (OtherActor :type Actor%20Object%20Reference)))

(event EventTick
  (params (DeltaSeconds :type Float%20%28single-precision%29)))

(event EventOnTrackEventTriggered
  (params (KeyFrameConfig :type Blackbird%20Track%20Event%20Key%20Frame%20Config%20Structure%20%28by%20ref%29) (OtherActor :type Actor%20Object%20Reference) (TriggerCount :type Integer%20%28by%20ref%29))
  (|SwitchGameplayTag (.KeyFrameTag (Utilities|Struct|BreakBlackbirdTrackEventKeyFrameConfig KeyFrameConfig))
    (:Track.Event.Start
      (CallFunction|OnSpawnSquadron)
      (Development|PrintString "spawn"))
    (:Track.Event.End
      (CallFunction|OnEndSquadron)
      (Development|PrintString "end"))))

(fn ConstructionScript)

(fn GetSplineStartLocation
  (params (Spline :type Spline%20Component%20Object%20Reference))
  (return (Spline|GetLocationatDistanceAlongSpline Spline 0.0 "World")))

(fn GetSplineStartRotation
  (params (Spline :type Spline%20Component%20Object%20Reference))
  (return (Spline|GetRotationatDistanceAlongSpline Spline 0.0 "Local")))

(fn GetSplineStartTransform
  (params (Spline :type Spline%20Component%20Object%20Reference))
  (return (Math|Transform|MakeTransform (CallFunction|GetSplineStartLocation Spline) (CallFunction|GetSplineStartRotation Spline))))

(fn SpawnSquadronCart
  (bind _returnvalue (Game|SpawnActorfromClass "/Game/Blueprints/Track/BP_Cart.BP_Cart_C" (CallFunction|GetSplineStartTransform (Variables|Default|GetEntrance%20Spline)) "Undefined" "MultiplyWithRoot" self (Variables|Default|GetEntrance%20Spline) (Variables|Default|GetEntrance%20Speed) true 0))
  (Class|BlackbirdCart|StartCart _returnvalue)
  (return _returnvalue))

(fn SpawnSquadronActor
  (params (Cart :type BP%20Cart%20Object%20Reference))
  (bind _returnvalue (Game|SpawnActorfromClass (Variables|Default|GetSquadron%20Class) (CallFunction|GetSplineStartTransform (Variables|Default|GetEntrance%20Spline)) "Undefined" "MultiplyWithRoot" Cart 0))
  (Transformation|AttachActorToActor _returnvalue Cart "None" "SnapToTarget" "SnapToTarget" "KeepRelative" true)
  (return _returnvalue))